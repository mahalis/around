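; Actor component that tracks health and alive state for its owner.
; TakeDamage subtracts health and returns whether the hit was lethal, clamping to zero and firing the Died dispatcher on death.
; Heal adds health up to MaximumHealth while alive and reports success; both record the time of the last health change on non-lethal changes.
; Reset restores full health and revives.
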(event EventBeginPlay)

(event EventTick
  (params (DeltaSeconds :type Float%20%28single-precision%29)))

(fn TakeDamage
  (params (Amount :type Integer))
  (if (Variables|Default|GetIsAlive)
    (if (> (- (Variables|Default|GetHealth) Amount) 0)
      (Variables|Default|SetHealth (- (Variables|Default|GetHealth) Amount))
      (Variables|Default|SetLastHealthChangeTime (Utilities|Time|GetGameTimeinSeconds))
      (return false)
      (else
        (Variables|Default|SetIsAlive false)
        (Default|CallDied)
        (Variables|Default|SetHealth 0)
        (return true)))))

(fn Heal
  (params (Amount :type Integer))
  (bind _maximumhealth (Variables|Default|GetMaximumHealth))
  (if (Variables|Default|GetIsAlive)
    (if (< (Variables|Default|GetHealth) _maximumhealth)
      (Variables|Default|SetHealth (Math|Integer|Min(Integer) (+ (Variables|Default|GetHealth) Amount) _maximumhealth))
      (Variables|Default|SetLastHealthChangeTime (Utilities|Time|GetGameTimeinSeconds))
      (return true)
      (else
        (return false)))))

(fn Reset
  (Variables|Default|SetHealth (Variables|Default|GetMaximumHealth))
  (Variables|Default|SetIsAlive true))