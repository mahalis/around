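; JamPlayerController is a player controller that handles camera look input and quitting the game.
; Pan and Tilt axes add scaled yaw and pitch directly, with Tilt inverted, while PanRate and TiltRate scale by world delta time for frame-rate-independent turning.
; Pressing Escape quits the game immediately.
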(event EventBeginPlay)

(event EventTick
  (params (DeltaSeconds :type Float%20%28single-precision%29)))

(event Input|AxisEvents|InputAxisPanRate
  (params (AxisValue :type Float%20%28single-precision%29))
  ;[1 1 1] camera controls
  (Class|PlayerController|AddYawInput (* AxisValue (Utilities|Time|GetWorldDeltaSeconds) 4e+01)))

(event Input|AxisEvents|InputAxisPan
  (params (AxisValue :type Float%20%28single-precision%29))
  ;[1 1 1] camera controls
  (Class|PlayerController|AddYawInput (* AxisValue 0.6)))

(event Input|AxisEvents|InputAxisTiltRate
  (params (AxisValue :type Float%20%28single-precision%29))
  ;[1 1 1] camera controls
  (Class|PlayerController|AddPitchInput (* AxisValue (Utilities|Time|GetWorldDeltaSeconds) 4e+01)))

(event Input|AxisEvents|InputAxisTilt
  (params (AxisValue :type Float%20%28single-precision%29))
  ;[1 1 1] camera controls
  (Class|PlayerController|AddPitchInput (* AxisValue -0.5)))

(event Input|KeyboardEvents|Escape
  (params (Key :type Key%20Structure :default "None"))
  (:Pressed
    (Game|QuitGame 0 "Quit" false)))

(fn ConstructionScript)