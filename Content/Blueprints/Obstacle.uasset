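; Obstacle actor with a collision box and mesh, configurable as thick or thin and tall or short.
; The construction script uses the Thick and Tall flags to scale the box and mesh width along Y and set their height along Z.
; A Hit function turns off collision and hides the mesh without destroying the actor.
; The event graph holds no active logic.
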(event EventBeginPlay)

(event Collision|EventActorBeginOverlap
  (params (OtherActor :type Actor%20Object%20Reference)))

(event EventTick
  (params (DeltaSeconds :type Float%20%28single-precision%29)))

(fn ConstructionScript
  (bind _tall (Variables|Default|GetTall))
  (bind _collision (Variables|Default|GetCollision))
  (bind _mesh (Variables|Default|GetMesh))
  (bind _thick (Variables|Default|GetThick))
  (bind _returnvalue (Components|Box|GetUnscaledBoxExtent _collision))
  (bind _relativescale3d (Variables|/Script/Engine.SceneComponent|GetRelativeScale3D _mesh))
  (Components|Box|SetBoxExtent _collision (Math|Vector|MakeVector (.x _returnvalue) (* (.y _returnvalue) (Math|Float|SelectFloat 1.0 0.3 _thick)) (Math|Float|SelectFloat 72.0 24.0 _tall)) false)
  (Transformation|SetRelativeScale3D _mesh (Math|Vector|MakeVector (.x _relativescale3d) (* (.y _relativescale3d) (Math|Float|SelectFloat 1.0 0.3 _thick)) (Math|Float|SelectFloat 1.5 0.5 _tall))))

(fn Hit
  (Collision|SetCollisionEnabled (Variables|Default|GetCollision) "NoCollision")
  (Rendering|SetVisibility (Variables|Default|GetMesh) false false))