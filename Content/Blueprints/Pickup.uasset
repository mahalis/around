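; Pickup actor that reports to the JamMode game mode when something overlaps it.
; It caches the game mode on BeginPlay and passes itself to RegisterHitPickup on any overlap, without filtering the other actor.
; PickedUp turns off the sphere's collision and hides the mesh rather than destroying the actor.
; SetMapPosition stores the pickup's row and index on the map.
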(event EventBeginPlay
  (bind _asjam_mode (Utilities|Casting|CastToJamMode (Game|GetGameMode)))
  (Variables|Default|SetMode _asjam_mode))

(event Collision|EventActorBeginOverlap
  (params (OtherActor :type Actor%20Object%20Reference))
  (Default|RegisterHitPickup (Variables|Default|GetMode) self))

(fn ConstructionScript)

(fn PickedUp
  (Collision|SetCollisionEnabled (Variables|Default|GetSphere) "NoCollision")
  (Rendering|SetVisibility (Variables|Default|GetMesh) false true))

(fn SetMapPosition
  (params (Row :type Integer) (Index :type Integer))
  (Variables|Default|SetRow Row)
  (Variables|Default|SetIndex Index))