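; Player character for a jam game that moves sideways across columns and jumps, with no forward movement of its own.
; Each tick it integrates custom gravity and side velocity, then applies each axis with a swept move, using hit normals to stop or land.
; Sideways position eases onto the nearest column when input and speed are low.
; Jumping is gated only by a cooldown, and animation rate follows game mode speed, slowing in air.
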(event EventBeginPlay
  (bind _asjam_mode (Utilities|Casting|CastToJamMode (Game|GetGameMode)))
  (Variables|Default|SetMode _asjam_mode))

(event EventTick
  (params (DeltaSeconds :type Float%20%28single-precision%29))
  (CallFunction|Move DeltaSeconds)
  (CallFunction|UpdateAnimation))

(event Input|ActionEvents|InputActionMainAction
  (params (Key :type Key%20Structure :default "None"))
  (:Pressed
    (Variables|Default|SetWantsJump true))
  (:Released
    (Variables|Default|SetWantsJump false)))

(event Input|KeyboardEvents|Escape
  (params (Key :type Key%20Structure :default "None"))
  (:Pressed
    (Game|QuitGame 0 "Quit" false)))

(fn ConstructionScript)

(fn Move
  (params (DeltaTime :type Float%20%28single-precision%29))
  (bind _returnvalue (Transformation|GetActorLocation))
  (CallFunction|UpdateUpVelocityandDesiredPosition DeltaTime)
  (CallFunction|UpdateSideVelocityandDesiredPosition DeltaTime)
  (Utilities|FlowControl|Sequence
    (:then_0
      (bind _sweephitresult (Transformation|SetActorLocation (Math|Vector|MakeVector (* (Variables|Default|GetSidePosition) (* (Variables|Default|GetMaxOffset) -1.0)) (.y _returnvalue) (.z _returnvalue)) true false)) ; move sideways
      (if (.bblockinghit _sweephitresult)
        (if (> (Math|Float|Absolute(Float) (.x (.normal _sweephitresult))) 0.7) ; is this a side collision?
          (Variables|Default|SetSideVelocity 0.0)
          (Variables|Default|SetSidePosition (/ (.x (.location _sweephitresult)) (* (Variables|Default|GetMaxOffset) -1.0))))))
    (:then_1
      (bind _sweephitresult_2 (Transformation|SetActorLocation (Math|Vector|MakeVector (.x _returnvalue) (.y _returnvalue) (Variables|Default|GetUpPosition)) true false))
      (if (.bblockinghit _sweephitresult_2)
        (if (> (.z (.normal _sweephitresult_2)) 0.7) ; falling?
          (Variables|Default|SetUpVelocity 0.0)
          (Variables|Default|SetUpPosition (.z (.location _sweephitresult_2)))
          (Variables|Default|SetInAir false))))))

(fn UpdateSideVelocityandDesiredPosition
  (params (DeltaTime :type Float%20%28single-precision%29))
  (bind _returnvalue (Input|AxisValues|GetMoveRight))
  (bind _maxspeed (Variables|Default|GetMaxSpeed))
  (bind _mode (Variables|Default|GetMode))
  (bind _maxoffset (Variables|Default|GetMaxOffset))
  (bind _returnvalue_2 (Math|Float|Absolute(Float) _returnvalue))
  (bind _columnspacing (Variables|/Game/Blueprints/JamMode.JamMode_C|GetColumnSpacing _mode))
  (bind _returnvalue_3 (> _returnvalue_2 0.1))
  (bind _returnvalue_4 (/ _maxoffset _columnspacing))
  (bind _output_get (Variables|Default|SetSideVelocity (Math|Float|SelectFloat (Math|Float|Clamp(Float) (+ (Variables|Default|GetSideVelocity) (* _returnvalue DeltaTime (Math|Float|SelectFloat 1e+01 5e+01 (Variables|Default|GetInAir)))) (* _maxspeed -1.0) _maxspeed) (* (Variables|Default|GetSideVelocity) (- 1.0 (* DeltaTime 1e+01))) _returnvalue_3)))
  (Variables|Default|SetSidePosition (Math|Float|SelectFloat (Math|Float|Clamp(Float) (+ (Variables|Default|GetSidePosition) (* _output_get DeltaTime)) -1.0) (Math|Interpolation|FInterpTo (Math|Float|Clamp(Float) (+ (Variables|Default|GetSidePosition) (* _output_get DeltaTime)) -1.0) (/ (Math|Conversions|ToFloat(Integer) (Math|Float|Round (* (Math|Float|Clamp(Float) (+ (Variables|Default|GetSidePosition) (* _output_get DeltaTime)) -1.0) _returnvalue_4))) _returnvalue_4) DeltaTime 1e+01) (or _returnvalue_3 (> (Math|Float|Absolute(Float) (Variables|Default|GetSideVelocity)) 2.0)))))

(fn UpdateUpVelocityandDesiredPosition
  (params (DeltaTime :type Float%20%28single-precision%29))
  (Variables|Default|SetUpVelocity (- (Variables|Default|GetUpVelocity) (* 2.4e+03 DeltaTime)))
  (if (and (CallFunction|CanJump) (Variables|Default|GetWantsJump))
    (CallFunction|Jump))
  (Variables|Default|SetUpPosition (+ (Variables|Default|GetUpPosition) (* (- (Variables|Default|GetUpVelocity) (* 2.4e+03 DeltaTime)) DeltaTime))))

(fn CanJump
  (return (> (Utilities|Time|GetGameTimeinSeconds) (+ (Variables|Default|GetLastJumpTime) 1.0))))

(fn Jump
  (Variables|Default|SetLastJumpTime (Utilities|Time|GetGameTimeinSeconds))
  (Variables|Default|SetUpVelocity (+ (Variables|Default|GetUpVelocity) 8e+02))
  (Variables|Default|SetInAir true))

(fn UpdateAnimation
  (Components|Timeline|SetPlayRate (Variables|Default|GetMesh) (Math|Float|SelectFloat 0.2 (/ (Variables|/Game/Blueprints/JamMode.JamMode_C|GetSpeed (Variables|Default|GetMode)) 6e+02) (Variables|Default|GetInAir))))